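; BP_Pasillo is the hallway controller for an anomaly-spotting loop, randomly picking a normal corridor or one of three anomalies.
; BeginPlay caches the Teleport, Door, TV2, LevelSign and Cat actors and resets the level sign.
; AnomalyS rolls the variant, triggers the door, TV or cat anomaly and sets HasAnomalies on the teleport.
; ResetAnomalies restores props whose flag is unset, while the default roll resets all three.
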(event Custom|AnomalyS
  (switch int (Math|Random|RandomIntegerinRange 0 3)
    (:0
      ;[1 1 1] DefaultMap
      (Development|PrintString "Default")
      (Default|ResetDoor (Utilities|Array|Get(acopy) (stale EventBeginPlay _outactors_2)))
      (Default|ResetTV2 (Utilities|Array|Get(acopy) (stale EventBeginPlay _outactors_3)))
      (Default|ResetCat (Utilities|Array|Get(acopy) (stale EventBeginPlay _outactors_5)))
      (Variables|/Game/Teleport.Teleport_C|SetHasAnomalies (Utilities|Array|Get(acopy) (stale EventBeginPlay _outactors)) false))
    (:1
      (Development|PrintString "A1")
      (Variables|Default|SetA2 false)
      (Variables|Default|SetA3 false)
      (Default|Anomaly1 (Utilities|Array|Get(acopy) (stale EventBeginPlay _outactors_2)))
      (Variables|/Game/Teleport.Teleport_C|SetHasAnomalies (Utilities|Array|Get(acopy) (stale EventBeginPlay _outactors)) true)
      (Variables|Default|SetA1 true)
      (CallFunction|ResetAnomalies))
    (:2
      (Development|PrintString "A2")
      (Variables|Default|SetA1 false)
      (Variables|Default|SetA3 false)
      (Default|Anomaly2 (Utilities|Array|Get(acopy) (stale EventBeginPlay _outactors_3)))
      (Variables|/Game/Teleport.Teleport_C|SetHasAnomalies (Utilities|Array|Get(acopy) (stale EventBeginPlay _outactors)) true)
      (Variables|Default|SetA2 true)
      (CallFunction|ResetAnomalies))
    (:3
      (Development|PrintString "A3")
      (Variables|Default|SetA1 false)
      (Variables|Default|SetA2 false)
      (Default|Anomaly3 (Utilities|Array|Get(acopy) (stale EventBeginPlay _outactors_5)))
      (Variables|/Game/Teleport.Teleport_C|SetHasAnomalies (Utilities|Array|Get(acopy) (stale EventBeginPlay _outactors)) true)
      (Variables|Default|SetA3 true)
      (CallFunction|ResetAnomalies))))

(event Custom|ResetAnomalies
  ;[1 1 1] Reset Anomalies
  (if (Variables|Default|GetA1)
    _
    (else
      (Default|ResetDoor (Utilities|Array|Get(acopy) (stale EventBeginPlay _outactors_2)))))
  (if (Variables|Default|GetA2)
    _
    (else
      (Default|ResetTV2 (Utilities|Array|Get(acopy) (stale EventBeginPlay _outactors_3)))))
  (if (not (Variables|Default|GetA3))
    (Default|ResetCat (Utilities|Array|Get(acopy) (stale EventBeginPlay _outactors_5)))))

(event EventBeginPlay
  (bind _outactors (Actor|GetAllActorsOfClass "/Game/Teleport.Teleport_C"))
  (bind _outactors_2 (Actor|GetAllActorsOfClass "/Game/Door.Door_C"))
  (bind _outactors_3 (Actor|GetAllActorsOfClass "/Game/TV2.TV2_C"))
  (bind _outactors_4 (Actor|GetAllActorsOfClass "/Game/LevelSign.LevelSign_C"))
  (Default|LevelReset (Utilities|Array|Get(acopy) _outactors_4))
  (bind _outactors_5 (Actor|GetAllActorsOfClass "/Game/Cat.Cat_C")))

(event Collision|EventActorBeginOverlap
  (params (OtherActor :type Actor%20Object%20Reference)))

(event EventTick
  (params (DeltaSeconds :type Float%20%28single-precision%29)))

(fn ConstructionScript)